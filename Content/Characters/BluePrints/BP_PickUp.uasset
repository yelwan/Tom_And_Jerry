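; BP_PickUp is a pickup actor that flags itself as owned when a qualifying actor overlaps its static mesh.
; On overlap it calls GetActorMessage on the other actor and sets IsOwned if the returned reference is valid.
; Its getter functions expose the pickup itself through GetPickUpElement, while the actor and enemy getters return nothing and GetPlayerAttacking returns false.
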(event OnComponentBeginOverlap(StaticMesh)
  (params (OverlappedComponent :type Primitive%20Component%20Object%20Reference) (OtherActor :type Actor%20Object%20Reference) (OtherComp :type Primitive%20Component%20Object%20Reference) (OtherBodyIndex :type Integer) (bFromSweep :type Boolean) (SweepResult :type Hit%20Result%20Structure%20%28by%20ref%29))
  (bind _target_actor (Class|BPIInteract|GetActor(Message) OtherActor))
  (Utilities|IsValid _target_actor
    (:Is%20Valid
      (Variables|Default|SetisOwned true))))

(event EventBeginPlay)

(event EventTick
  (params (DeltaSeconds :type Float%20%28single-precision%29)))

(fn ConstructionScript)

(fn GetActor
  (return 0))

(fn GetEnemyActor
  (return 0))

(fn GetPickUpElement
  (return self))

(fn GetPlayerAttacking
  (return false))