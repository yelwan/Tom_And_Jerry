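; Behavior tree task that makes an enemy flee from the first player character.
; Each AI tick, it gets the enemy actor from the controlled pawn via a message call and projects a point directly away from the player at the enemy's own height.
; It then issues an AI MoveTo toward a random reachable navmesh point around that spot.
; The task never calls Finish Execute.
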(event EventReceiveTickAI
  (params (OwnerController :type AI%20Controller%20Object%20Reference) (ControlledPawn :type Pawn%20Object%20Reference) (DeltaSeconds :type Float%20%28single-precision%29))
  (bind _target_actor_ai (Class|BPIInteract|GetEnemyActor(Message) ControlledPawn))
  (Utilities|IsValid _target_actor_ai
    (:Is%20Valid
      (AI|AIMoveTo _target_actor_ai (.RandomLocation (AI|Navigation|GetRandomReachablePointinRadius (Math|Vector|MakeVector (.x (+ (Transformation|GetActorLocation _target_actor_ai) (* (Math|Vector|GetForwardVector (Math|Rotator|FindLookatRotation (Transformation|GetActorLocation _target_actor_ai) (Transformation|GetActorLocation (Game|GetPlayerCharacter 0)))) -5e+02))) (.y (+ (Transformation|GetActorLocation _target_actor_ai) (* (Math|Vector|GetForwardVector (Math|Rotator|FindLookatRotation (Transformation|GetActorLocation _target_actor_ai) (Transformation|GetActorLocation (Game|GetPlayerCharacter 0)))) -5e+02))) (.Z (Math|Vector|BreakVector (Transformation|GetActorLocation _target_actor_ai)))) 5e+02 0 0)) 0 5.0 false))))