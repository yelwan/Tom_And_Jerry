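; Enemy AI controller that runs the enemy behavior tree and tells it when the player has been detected.
; On both BeginPlay and Possess it starts BT_Enemy, stores the player character in the blackboard and binds the AI perception update.
; A perception update for the player sets the detected flag to true without checking sensing success, so this controller never clears it.
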(event Custom|On%20Target%20Perception%20Updated
  (params (Actor :type Actor%20Object%20Reference) (Stimulus :type AI%20Stimulus%20Structure))
  (if (== Actor (Game|GetPlayerCharacter 0))
    (AI|Components|Blackboard|SetValueasBool (AI|GetBlackboard 0) (Variables|Default|GetBB_Player_Detected) true)))

(event EventTick
  (params (DeltaSeconds :type Float%20%28single-precision%29)))

(event EventPossess
  (params (PossessedPawn :type Pawn%20Object%20Reference))
  (Utilities|FlowControl|Sequence
    (:then_0
      (AI|RunBehaviorTree "/Game/Characters/BluePrints/AI/BT_Enemy.BT_Enemy")
      (AI|Components|Blackboard|SetValueasObject (AI|GetBlackboard 0) (Variables|Default|GetBB_Player) (Game|GetPlayerCharacter 0)))
    (:then_1
      (EventDispatchers|AssignOnTargetPerceptionUpdated (Variables|Default|GetAIPerception) (delegate Custom|On%20Target%20Perception%20Updated)))))

(event EventBeginPlay
  (Utilities|FlowControl|Sequence
    (:then_0
      (AI|RunBehaviorTree "/Game/Characters/BluePrints/AI/BT_Enemy.BT_Enemy")
      (AI|Components|Blackboard|SetValueasObject (AI|GetBlackboard 0) (Variables|Default|GetBB_Player) (Game|GetPlayerCharacter 0)))
    (:then_1
      (EventDispatchers|AssignOnTargetPerceptionUpdated (Variables|Default|GetAIPerception) (delegate Custom|On%20Target%20Perception%20Updated)))))

(fn ConstructionScript)