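; AI-controlled Jerry character that attacks the player with leaps, damaging hits and thrown objects.
; JumpAttack predicts the player's position from horizontal velocity, launches the character on a suggested projectile arc and stops movement on landing.
; Jump and regular attack damage events apply fixed amounts while CanApplyDamage is set.
; ShootPlayer detaches a carried actor and impulses its mesh using a moving-target velocity solution aimed at the player.
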(event Custom|OnLand
  (params (Hit :type Hit%20Result%20Structure%20%28by%20ref%29))
  (EventDispatchers|UnbindEventfromLandedDelegate (delegate Custom|OnLand))
  (Components|Movement|StopMovementImmediately (Variables|Character|GetCharacterMovement)))

(event Custom|Shoot%20Player
  (params (Target%20Actor :type Actor%20Object%20Reference) (Shooted%20Actor :type BP%20Pick%20Up%20Object%20Reference))
  (if (Variables|Default|GetisCarrying)
    (Transformation|DetachFromActor Shooted%20Actor "KeepWorld" "KeepWorld" "KeepWorld")
    (bind _outlaunchvelocity (Class|GameplayStatics|SuggestProjectileVelocityMovingTarget (Transformation|GetActorLocation Shooted%20Actor) (Game|GetPlayerCharacter 0) "0, 0, 0" -2.0 1.0 "None" 0.0))
    (Physics|AddImpulse (Variables|/Game/Characters/BluePrints/BP_PickUp.BP_PickUp_C|GetStaticMesh Shooted%20Actor) _outlaunchvelocity "None" true)
    (Variables|Default|SetisCarrying false)
    (Variables|/Game/Characters/BluePrints/BP_PickUp.BP_PickUp_C|SetisOwned Shooted%20Actor false)))

(event EventBeginPlay
  (|CallParentFunction) ; This node is disabled and will not be called.\nDrag off pins to build functionality.
)

(event Collision|EventActorBeginOverlap
  (params (OtherActor :type Actor%20Object%20Reference))
  (|CallParentFunction OtherActor) ; This node is disabled and will not be called.\nDrag off pins to build functionality.
)

(event EventTick
  (params (DeltaSeconds :type Float%20%28single-precision%29))
  (|CallParentFunction DeltaSeconds) ; This node is disabled and will not be called.\nDrag off pins to build functionality.
)

(event EventDeactivateDamage
  (params (Target%20Actor :type Actor%20Object%20Reference))
  (Variables|Default|SetCan%20Apply%20Damage false))

(event EventDamageJumpAttack
  (params (Target%20Actor :type Actor%20Object%20Reference))
  (if (Variables|Default|GetCan%20Apply%20Damage)
    (Game|Damage|ApplyDamage Target%20Actor 35.0 0 0 "/Script/Engine.DamageType")))

(event EventDamageAttack
  (params (Target%20Actor :type Actor%20Object%20Reference))
  (if (Variables|Default|GetCan%20Apply%20Damage)
    (Game|Damage|ApplyDamage Target%20Actor 2e+01 0 0 "/Script/Engine.DamageType")))

(event EventJumpAttack
  (params (TargetActor :type Character%20Object%20Reference))
  (bind _targetlocation (CallFunction|CalculateBestMove (Game|GetPlayerCharacter 0) 1.0))
  (bind _outlaunchvelocity (Game|SuggestProjectileVelocityCustomArc (Transformation|GetActorLocation) (Math|Vector|MakeVector (.x _targetlocation) (.y _targetlocation) (.z _targetlocation)) 0.0 0.5))
  (|CallParentFunction TargetActor)
  (Character|LaunchCharacter _outlaunchvelocity true true)
  (EventDispatchers|BindEventtoLandedDelegate (delegate Custom|OnLand)))

(fn ConstructionScript
  (|CallParentFunction))

(fn CalculateBestMove
  (params (TargetActor :type Character%20Object%20Reference) (Time :type Float%20%28double-precision%29))
  (return (+ (Transformation|GetActorLocation TargetActor) (* (* (Transformation|GetVelocity TargetActor) "1.000000,1.000000,0.000000") Time))))

(fn GetActor
  (return self))

(fn GetEnemyActor
  (return self))

(fn GetPickUpElement
  (return 0))

(fn GetPlayerAttacking
  (return false))