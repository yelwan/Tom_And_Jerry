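; Base character Blueprint providing a player attack and an enemy attack that share one counter-punch montage.
; Attack locks player input for the montage's length and fires a short forward debug trace whose result is unused.
; EnemyAttack launches the character using CalculateBestMove, which extrapolates the player's horizontal position over AnimLength and adds height.
; That world position is passed directly as launch velocity, and only Attack sets AnimLength.
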(event Custom|Enemy%20Attack
  (bind _location (CallFunction|CalculateBestMove (Game|GetPlayerCharacter 0) (Variables|Default|GetAnimLength)))
  (Animation|PlayAnimMontage "/Game/Characters/tom/Mesh/Animations/Combat_Animations/Paired_CounterPunch_PalmStrike_Att_Montage.Paired_CounterPunch_PalmStrike_Att_Montage" 1.0 "None")
  (Character|LaunchCharacter _location true true))

(event Custom|Attack
  (Input|DisableInput (Game|GetPlayerController 0))
  (bind _returnvalue (Animation|PlayAnimMontage "/Game/Characters/tom/Mesh/Animations/Combat_Animations/Paired_CounterPunch_PalmStrike_Att_Montage.Paired_CounterPunch_PalmStrike_Att_Montage" 1.0 "None"))
  (Variables|Default|SetAnimLength _returnvalue)
  (Collision|LineTraceByChannel (Transformation|GetActorLocation) (+ (Transformation|GetActorLocation) (* (Transformation|GetActorForwardVector) 47.0)) "TraceTypeQuery1" false 0 "ForDuration")
  (Utilities|FlowControl|Delay (Variables|Default|GetAnimLength))
  (Input|EnableInput (Game|GetPlayerController 0)))

(event EventBeginPlay)

(event Collision|EventActorBeginOverlap
  (params (OtherActor :type Actor%20Object%20Reference)))

(event EventTick
  (params (DeltaSeconds :type Float%20%28single-precision%29)))

(fn ConstructionScript)

(fn CalculateBestMove
  (params (Actor :type Actor%20Object%20Reference) (Time :type Float%20%28double-precision%29))
  (return (+ (+ (* (* (Transformation|GetVelocity Actor) "1.000000,1.000000,0.000000") Time) (Transformation|GetActorLocation Actor)) "0.000000,0.000000,100.000000")))